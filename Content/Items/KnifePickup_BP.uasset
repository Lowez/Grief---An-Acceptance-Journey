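; Knife pickup actor that refills the player's projectile count.
; When a Player_BP overlaps its sphere and is not already at max projectiles, it adds a fixed amount, clamped to the player's maximum.
; It then refreshes the projectile HUD, plays a 2D pickup sound and destroys itself.
; At max projectiles, the pickup stays in the world.
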(event `self.Sphere.OnComponentBeginOverlap`
  (params (OverlappedComponent :type "PrimitiveComponent Object Reference") (OtherActor :type "Actor Object Reference") (OtherComp :type "PrimitiveComponent Object Reference") (OtherBodyIndex :type Integer) (bFromSweep :type Boolean) (SweepResult :type "HitResult Structure (by ref)"))
  (bind _as_player_bp (`self.As Player BP`))
  (bind _asplayer_bp (cast `/Game/PlayerCharacter/Player_BP` OtherActor))
  (bind _output_get (set `self.As Player BP` _asplayer_bp))
  (if (not (== (`/Game/PlayerCharacter/Player_BP.projectiles` _output_get) (`/Game/PlayerCharacter/Player_BP.maxProjectiles` _output_get)))
    (set `/Game/PlayerCharacter/Player_BP.projectiles` (`KismetMathLibrary.Clamp` (+ (`/Game/PlayerCharacter/Player_BP.projectiles` _as_player_bp) 5) 1 (`/Game/PlayerCharacter/Player_BP.maxProjectiles` _as_player_bp)) _as_player_bp)
    (`/Game/WidgetBlueprints/PlayerHUD_WB.UpdateHUDProjectiles` (`/Game/PlayerCharacter/Player_BP.HUDref` (`self.As Player BP`)))
    (`GameplayStatics.SpawnSound2D` "/Game/Sounds/SFX/pickup_sound.pickup_sound" 1.0 1.0 0.0 null)
    (`self.K2_DestroyActor`)))

(fn `UserConstructionScript`)