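; Boss character that chases the player along X, turns to face them, and attacks with melee or paired fireballs.
; Overlap boxes start looping randomized timers that jump the animation instance to attack nodes; separate events perform the melee line trace and spawn aimed projectiles.
; Damage updates a health bar widget, knocks the boss back, briefly blocks attacks and later sets flying movement, or plays death and destroys it at zero health.
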(event `self.ReceiveBeginPlay`
  (set `self.maxHealth` (`self.health`))
  (bind _returnvalue (`|CreateWidget` "/Game/WidgetBlueprints/BossHealthBar_WB.BossHealthBar_WB_C" null self))
  (bind _output_get (set `self.bossHealthBar` _returnvalue))
  (`UserWidget.AddToViewport` _output_get 0))

(event `self.ReceiveTick`
  (params (DeltaSeconds :type "Float (single-precision)"))
  (bind (_returnvalue_x _returnvalue_y _returnvalue_z) (`KismetMathLibrary.BreakVector` (- (`self.K2_GetActorLocation` (`GameplayStatics.GetPlayerCharacter` 0)) (`self.K2_GetActorLocation`))))
  (bind _returnvalue_x_2 (`KismetMathLibrary.BreakVector` (`KismetMathLibrary.Normal` (`KismetMathLibrary.MakeVector` _returnvalue_x _returnvalue_y _returnvalue_z))))
  (if (not (`self.isdead`))
    (`self.handlerotation`)
    (if (not (< (`KismetMathLibrary.Abs` _returnvalue_x) 800.0))
      (`self.AddMovementInput` (1.0 0.0 0.0) _returnvalue_x_2))))

(event `handlerotation`
  (bind _returnvalue_x (`KismetMathLibrary.BreakVector` (`KismetMathLibrary.GetDirectionUnitVector` (`self.K2_GetActorLocation` (`GameplayStatics.GetPlayerCharacter` 0)) (`self.K2_GetActorLocation`))))
  ;[1 1 1] HandleRotation
  (if (`self.isdead`)
    _
    (elif (< _returnvalue_x 0.0)
      (`self.K2_SetActorRotation` (struct))
      (else
        (`self.K2_SetActorRotation` (struct :`Yaw` 180.0))))))

(event `meleeAttack`
  (if (not (or (`self.isAttacking`) (`self.isdead`)))
    (set `self.isAttacking` true)
    (`PaperZDAnimInstance.JumpToNode` (`PaperZDAnimationComponent.AnimInstance` (`self.AnimationComponent`)) "MeleeAttack" "None")
    (set `self.isAttacking` false)))

(event `self.Box.OnComponentBeginOverlap`
  (params (OverlappedComponent :type "PrimitiveComponent Object Reference") (OtherActor :type "Actor Object Reference") (OtherComp :type "PrimitiveComponent Object Reference") (OtherBodyIndex :type Integer) (bFromSweep :type Boolean) (SweepResult :type "HitResult Structure (by ref)"))
  (if (== OtherActor (`GameplayStatics.GetPlayerCharacter` 0))
    (set `self.meleeActive` true)
    (set `self.attackMode` true)
    (bind _returnvalue (`KismetSystemLibrary.K2_SetTimerDelegate` (delegate `meleeAttack`) (`KismetMathLibrary.RandomFloatInRange` 2.0 4.0) true))
    (set `self.meleeEvent` _returnvalue)))

(event `melee`
  (bind _returnvalue (`self.K2_GetActorLocation`))
  (bind (_returnvalue_x _returnvalue_y) (`KismetMathLibrary.BreakVector` (`self.GetActorForwardVector`)))
  ;[1 1 1] MeleeAttack
  (bind _outhit (`KismetSystemLibrary.LineTraceSingleForObjects` _returnvalue (+ _returnvalue (* (`KismetMathLibrary.MakeVector` _returnvalue_x _returnvalue_y -200.0) (500.0 0.0 1.0))) (`|MakeArray` "ObjectTypeQuery3" :!type "EObjectTypeQuery Enum")))
  (bind (_bblockinghit _binitialoverlap _time _distance _location _impactpoint _normal _impactnormal _physmat _hitactor) (`GameplayStatics.BreakHitResult` _outhit))
  (if (== _hitactor (`GameplayStatics.GetPlayerCharacter` 0))
    (`GameplayStatics.ApplyDamage` _hitactor 1.0)))

(event `self.BoxRanged.OnComponentBeginOverlap`
  (params (OverlappedComponent :type "PrimitiveComponent Object Reference") (OtherActor :type "Actor Object Reference") (OtherComp :type "PrimitiveComponent Object Reference") (OtherBodyIndex :type Integer) (bFromSweep :type Boolean) (SweepResult :type "HitResult Structure (by ref)"))
  (if (== OtherActor (`GameplayStatics.GetPlayerCharacter` 0))
    (set `self.rangedActive` true)
    (set `self.attackMode` true)
    (bind _returnvalue (`KismetSystemLibrary.K2_SetTimerDelegate` (delegate `rangedAttack`) (`KismetMathLibrary.RandomFloatInRange` 2.0 4.0) true))
    (set `self.rangedEvent` _returnvalue)))

(event `LaunchFireballs`
  (bind _returnvalue (`KismetMathLibrary.FindLookAtRotation` (`self.K2_GetActorLocation`) (`self.K2_GetActorLocation` (`GameplayStatics.GetPlayerCharacter` 0))))
  ;[1 1 1] RangedAttack
  (`/Engine/EditorBlueprintResources/StandardMacros.DoOnce` false :!label _label
    (:`Completed`
      (`SceneComponent.K2_SetWorldRotation` (`self.fireball1spawn`) _returnvalue false false)
      (`|SpawnActorFromClass` "/Game/Bosses/Boss1/Blueprints/BossProjectile_BP.BossProjectile_BP_C" (`SceneComponent.K2_GetComponentToWorld` (`self.fireball1spawn`)) "Undefined" "OverrideRootScale" null null)
      (`SceneComponent.K2_SetWorldRotation` (`self.fireball2spawn`) _returnvalue false false)
      (`|SpawnActorFromClass` "/Game/Bosses/Boss1/Blueprints/BossProjectile_BP.BossProjectile_BP_C" (`SceneComponent.K2_GetComponentToWorld` (`self.fireball2spawn`)) "Undefined" "OverrideRootScale" null null)
      (`KismetSystemLibrary.Delay` 1.0)
      (goto _label :!via `Reset`))))

(event `rangedAttack`
  (if (not (or (`self.isAttacking`) (`self.isdead`)))
    (set `self.isAttacking` true)
    (`PaperZDAnimInstance.JumpToNode` (`PaperZDAnimationComponent.AnimInstance` (`self.AnimationComponent`)) "RangedAttack" "None")
    (set `self.isAttacking` false)))

(event `self.Box.OnComponentEndOverlap`
  (params (OverlappedComponent :type "PrimitiveComponent Object Reference") (OtherActor :type "Actor Object Reference") (OtherComp :type "PrimitiveComponent Object Reference") (OtherBodyIndex :type Integer))
  (if (== OtherActor (`GameplayStatics.GetPlayerCharacter` 0))
    (set `self.meleeActive` false)
    (`KismetSystemLibrary.K2_ClearAndInvalidateTimerHandle` (`self.meleeEvent`))))

(event `self.BoxRanged.OnComponentEndOverlap`
  (params (OverlappedComponent :type "PrimitiveComponent Object Reference") (OtherActor :type "Actor Object Reference") (OtherComp :type "PrimitiveComponent Object Reference") (OtherBodyIndex :type Integer))
  (if (== OtherActor (`GameplayStatics.GetPlayerCharacter` 0))
    (set `self.rangedActive` false)
    (set `self.attackMode` false)
    (`KismetSystemLibrary.K2_ClearAndInvalidateTimerHandle` (`self.rangedEvent`))))

(event `self.ReceiveAnyDamage`
  (params (Damage :type "Float (single-precision)") (DamageType :type "DamageType Object Reference") (InstigatedBy :type "Controller Object Reference") (DamageCauser :type "Actor Object Reference"))
  (bind _returnvalue_x (`KismetMathLibrary.BreakVector` (`KismetMathLibrary.GetDirectionUnitVector` (`self.K2_GetActorLocation` DamageCauser) (`self.K2_GetActorLocation`))))
  (bind _animinstance (`PaperZDAnimationComponent.AnimInstance` (`self.AnimationComponent`)))
  (set `self.health` (- (`self.health`) Damage))
  (set `self.isAttacking` true)
  (`/Game/WidgetBlueprints/BossHealthBar_WB.UpdateHealthBar` (`self.bossHealthBar`))
  (`self.LaunchCharacter` (`KismetMathLibrary.MakeVector` (* (select `bool` (< _returnvalue_x 0.0) :`false` -1.0 :`true` 1.0) -800.0) 0.0 150.0))
  (`|ExecutionSequence`
    (:`then_0`
      (if (<= (`self.health`) 0.0)
        (set `self.isdead` true)
        (`Widget.RemoveFromParent` (`self.bossHealthBar`))
        (`PaperZDAnimInstance.JumpToNode` _animinstance "Death" "None")
        (`KismetSystemLibrary.Delay` 1.5)
        (`self.K2_DestroyActor`)
        (else
          (`PaperZDAnimInstance.JumpToNode` _animinstance "Damaged" "None")
          (`KismetSystemLibrary.RetriggerableDelay` 1.0)
          (set `self.isAttacking` false))))
    (:`then_1`
      (`KismetSystemLibrary.Delay` 0.7)
      (`CharacterMovementComponent.SetMovementMode` (`self.CharacterMovement`) "MOVE_Flying" 0))))

(fn `UserConstructionScript`)