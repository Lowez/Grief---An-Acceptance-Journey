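; Side-scrolling hound enemy that patrols along X, attacks the player and shows a health bar when hurt.
; Forward and downward traces detect obstacles and ledges, sharing a DoOnce that pauses then reverses movement.
; A box overlap halts patrol and loops a timer playing attack animations, while a separate Attack event traces and applies damage.
; Taking damage turns it toward the attacker with knockback and a brief stun, or destroys it at zero health.
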(event `self.ReceiveBeginPlay`
  (set `CharacterMovementComponent.MaxWalkSpeed` (`self.Velocidade Máxima Para Caminhar`) (`self.CharacterMovement`))
  (set `self.maxhealth` (`self.health`))
  (bind _asenemy_health_bar_wb (cast `/Game/WidgetBlueprints/EnemyHealthBar_WB` (`WidgetComponent.GetWidget` (`self.Widget`))))
  (set `self.As Enemy Health Bar WB` _asenemy_health_bar_wb)
  (set `/Game/WidgetBlueprints/EnemyHealthBar_WB.houndreference` self _asenemy_health_bar_wb))

(event `Handlerotation`
  ;[1 1 1] Handle Rotation
  (if (> (`self.movementdirection`) 0.0)
    (`self.K2_SetActorRotation` (struct))
    (else
      (`self.K2_SetActorRotation` (struct :`Yaw` 180.0)))))

(event `self.ReceiveTick`
  (params (DeltaSeconds :type "Float (single-precision)"))
  (`self.Handlerotation`)
  (`self.Handlemovement`))

(event `Handlemovement`
  (bind _returnvalue (`self.K2_GetActorLocation`))
  (bind _returnvalue_2 (`self.K2_GetActorLocation`))
  ;[1 1 1] Handle Movement
  (if (not (or (`self.isdead`) (`self.enemydamaged`) (`NavMovementComponent.IsFalling` (`self.CharacterMovement`)) (`self.attackMode`)))
    (`self.AddMovementInput` (1.0 0.0 0.0) (`self.movementdirection`))
    (`|ExecutionSequence`
      (:`then_0`
        ;;[1 1 1] Detect object in front of the enemy
        (bind (_outhit _returnvalue_3) (`KismetSystemLibrary.LineTraceSingleForObjects` _returnvalue (+ _returnvalue (* (`self.GetActorForwardVector`) (100.0 0.0 0.0))) (`|MakeArray` "ObjectTypeQuery1" "ObjectTypeQuery2" "ObjectTypeQuery3" :!type "EObjectTypeQuery Enum") false (`|MakeArray` (`GameplayStatics.GetPlayerCharacter` 0) :!type "Actor Object Reference")))
        (if _returnvalue_3
          (`/Engine/EditorBlueprintResources/StandardMacros.DoOnce` false :!label _label
            (:`Completed`
              (set `CharacterMovementComponent.MaxWalkSpeed` 0.0 (`self.CharacterMovement`))
              (`KismetSystemLibrary.Delay` (`self.waitTime`))
              (set `CharacterMovementComponent.MaxWalkSpeed` (`self.Velocidade Máxima Para Caminhar`) (`self.CharacterMovement`))
              (set `self.movementdirection` (* (`self.movementdirection`) -1.0))
              (goto _label :!via `Reset`)))))
      (:`then_1`
        ;;[1 1 1] Detect if enemy is on the edge of the world
        (bind (_outhit_2 _returnvalue_4) (`KismetSystemLibrary.LineTraceSingleForObjects` _returnvalue_2 (+ (- _returnvalue_2 (0.0 0.0 100.0)) (* (`self.GetActorForwardVector`) (100.0 0.0 0.0))) (`|MakeArray` "ObjectTypeQuery1" "ObjectTypeQuery2" "ObjectTypeQuery3" :!type "EObjectTypeQuery Enum") false (`|MakeArray` (`GameplayStatics.GetPlayerCharacter` 0) :!type "Actor Object Reference")))
        (if (not _returnvalue_4)
          (goto _label))))))

(event `self.ReceiveAnyDamage`
  (params (Damage :type "Float (single-precision)") (DamageType :type "DamageType Object Reference") (InstigatedBy :type "Controller Object Reference") (DamageCauser :type "Actor Object Reference"))
  (bind _returnvalue_x (`KismetMathLibrary.BreakVector` (`KismetMathLibrary.GetDirectionUnitVector` (`self.K2_GetActorLocation` DamageCauser) (`self.K2_GetActorLocation`))))
  (bind _returnvalue (select `bool` (< _returnvalue_x 0.0) :`false` -1.0 :`true` 1.0))
  ;[1 1 1] TakeDamageEvent
  (set `self.health` (- (`self.health`) Damage))
  (`/Game/WidgetBlueprints/EnemyHealthBar_WB.UpdateHealthBar` (`self.As Enemy Health Bar WB`))
  (set `self.enemydamaged` true)
  (set `self.movementdirection` _returnvalue)
  (`PaperZDAnimInstance.JumpToNode` (`PaperZDAnimationComponent.AnimInstance` (`self.AnimationComponent`)) (`self.DamagedJumpNode`) "None")
  (if (<= (`self.health`) 0.0)
    (set `self.isdead` true)
    (`SceneComponent.SetVisibility` (`self.Widget`) false false)
    (`PrimitiveComponent.SetCollisionProfileName` (`self.CapsuleComponent`) "OverlapOnlyPawn" true)
    (`KismetSystemLibrary.Delay` 0.2)
    (`self.K2_DestroyActor`)
    (else
      (`self.LaunchCharacter` (`KismetMathLibrary.MakeVector` (* _returnvalue -800.0) 0.0 150.0))
      (`SceneComponent.SetVisibility` (`self.Widget`) true false)
      (`KismetSystemLibrary.RetriggerableDelay` 1.0)
      (set `self.enemydamaged` false))))

(event `self.Box.OnComponentBeginOverlap`
  (params (OverlappedComponent :type "PrimitiveComponent Object Reference") (OtherActor :type "Actor Object Reference") (OtherComp :type "PrimitiveComponent Object Reference") (OtherBodyIndex :type Integer) (bFromSweep :type Boolean) (SweepResult :type "HitResult Structure (by ref)"))
  ;[1 1 1] Detects if player got infront of enemy
  (if (== OtherActor (`GameplayStatics.GetPlayerCharacter` 0))
    (set `self.attackMode` true)
    (bind _returnvalue (`KismetSystemLibrary.K2_SetTimerDelegate` (delegate `houndAttack`) 1.0 true))
    (set `self.attackEvent` _returnvalue)))

(event `self.Box.OnComponentEndOverlap`
  (params (OverlappedComponent :type "PrimitiveComponent Object Reference") (OtherActor :type "Actor Object Reference") (OtherComp :type "PrimitiveComponent Object Reference") (OtherBodyIndex :type Integer))
  ;[1 1 1] Ends attack repeat if player leaves the colision box
  (if (== OtherActor (`GameplayStatics.GetPlayerCharacter` 0))
    (set `self.attackMode` false)
    (`KismetSystemLibrary.K2_ClearAndInvalidateTimerHandle` (`self.attackEvent`))))

(event `houndAttack`
  ;[1 1 1] Detects if player got infront of enemy
  (`PaperZDAnimInstance.JumpToNode` (`PaperZDAnimationComponent.AnimInstance` (`self.AnimationComponent`)) (`self.AttackJumpNode`) "None"))

(event `Attack`
  (bind _returnvalue (`self.K2_GetActorLocation`))
  ;[1 1 1] Enemy Attack custom event
  (bind _outhit (`KismetSystemLibrary.LineTraceSingleForObjects` _returnvalue (+ _returnvalue (* (`self.GetActorForwardVector`) (125.0 0.0 0.0))) (`|MakeArray` "ObjectTypeQuery3" :!type "EObjectTypeQuery Enum")))
  (bind (_bblockinghit _binitialoverlap _time _distance _location _impactpoint _normal _impactnormal _physmat _hitactor) (`GameplayStatics.BreakHitResult` _outhit))
  (if (== _hitactor (`GameplayStatics.GetPlayerCharacter` 0))
    (`GameplayStatics.ApplyDamage` _hitactor 1.0)))

(fn `UserConstructionScript`)