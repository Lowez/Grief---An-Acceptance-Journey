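; Enemy fireball projectile that damages the player and explodes when its sphere begins an overlap.
; Overlapping the player applies damage on every overlap, then passes through a DoOnce into the explosion; actors tagged "level" jump straight to the explosion, bypassing the DoOnce.
; The explosion swaps the Paper2D flipbook, waits for its length, then destroys the actor.
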(event `self.Sphere.OnComponentBeginOverlap`
  (params (OverlappedComponent :type "PrimitiveComponent Object Reference") (OtherActor :type "Actor Object Reference") (OtherComp :type "PrimitiveComponent Object Reference") (OtherBodyIndex :type Integer) (bFromSweep :type Boolean) (SweepResult :type "HitResult Structure (by ref)"))
  (bind _returnvalue (`GameplayStatics.GetPlayerCharacter` 0))
  (if (== OtherActor _returnvalue)
    (`GameplayStatics.ApplyDamage` _returnvalue 1.0)
    (`/Engine/EditorBlueprintResources/StandardMacros.DoOnce` false
      (:`Completed`
        (`PaperFlipbookComponent.SetFlipbook` (`self.PaperFlipbook`) "/Game/DemonEnemy/FlipBooks/Attack/fire-ball-explodes-fp.fire-ball-explodes-fp" :!label _label)
        (`KismetSystemLibrary.Delay` (`PaperFlipbookComponent.GetFlipbookLength` (`self.PaperFlipbook`)))
        (`self.K2_DestroyActor`)))
    (elif (`self.ActorHasTag` OtherActor "level")
      (goto _label))))

(fn `UserConstructionScript`)