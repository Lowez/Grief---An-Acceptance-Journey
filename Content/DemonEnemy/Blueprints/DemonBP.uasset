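; Ranged demon enemy that turns along the X axis to face the player every tick until it dies.
; While the player is inside its Box trigger, a looping timer plays the attack animation when grounded; a separate SpawnProjectile event fires from SpawnFireball.
; Damage updates a health bar widget, then either jumps to a hurt animation with knockback and briefly shows the bar, or plays death and destroys the actor.
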(event `self.ReceiveBeginPlay`
  (set `self.maxHealth` (`self.health`))
  (bind _asranged_enemy_health_bar_wb (cast `/Game/WidgetBlueprints/RangedEnemyHealthBar_WB` (`WidgetComponent.GetWidget` (`self.Widget`))))
  (bind _output_get (set `self.As Ranged Enemy Health Bar WB` _asranged_enemy_health_bar_wb))
  (set `/Game/WidgetBlueprints/RangedEnemyHealthBar_WB.DemonRef` self _output_get))

(event `self.ReceiveTick`
  (params (DeltaSeconds :type "Float (single-precision)"))
  (`self.handlerotation`))

(event `handlerotation`
  (bind _returnvalue_x (`KismetMathLibrary.BreakVector` (`KismetMathLibrary.GetDirectionUnitVector` (`self.K2_GetActorLocation` (`GameplayStatics.GetPlayerCharacter` 0)) (`self.K2_GetActorLocation`))))
  ;[1 1 1] HandleRotation
  (if (`self.isdead`)
    _
    (elif (< _returnvalue_x 0.0)
      (`self.K2_SetActorRotation` (struct))
      (else
        (`self.K2_SetActorRotation` (struct :`Yaw` 180.0))))))

(event `self.ReceiveAnyDamage`
  (params (Damage :type "Float (single-precision)") (DamageType :type "DamageType Object Reference") (InstigatedBy :type "Controller Object Reference") (DamageCauser :type "Actor Object Reference"))
  (bind _returnvalue_x (`KismetMathLibrary.BreakVector` (`KismetMathLibrary.GetDirectionUnitVector` (`self.K2_GetActorLocation` DamageCauser) (`self.K2_GetActorLocation`))))
  (bind _animinstance (`PaperZDAnimationComponent.AnimInstance` (`self.AnimationComponent`)))
  ;[1 1 1] TakeDamageEvent
  (set `self.health` (- (`self.health`) Damage))
  (`/Game/WidgetBlueprints/RangedEnemyHealthBar_WB.UpdateHealthBar` (`self.As Ranged Enemy Health Bar WB`))
  (set `self.enemydamaged` true)
  (if (<= (`self.health`) 0.0)
    (`PaperZDAnimInstance.JumpToNode` _animinstance (`self.DieJumpNode`) "None")
    (set `self.isdead` true)
    (`SceneComponent.SetVisibility` (`self.Widget`) false false)
    (`PrimitiveComponent.SetCollisionProfileName` (`self.CapsuleComponent`) "OverlapOnlyPawn" true)
    (`KismetSystemLibrary.Delay` 0.3)
    (`self.K2_DestroyActor`)
    (else
      (`PaperZDAnimInstance.JumpToNode` _animinstance (`self.DamagedJumpNode`) "None")
      (`self.LaunchCharacter` (`KismetMathLibrary.MakeVector` (* (select `bool` (< _returnvalue_x 0.0) :`false` -1.0 :`true` 1.0) -800.0) 0.0 150.0))
      (`SceneComponent.SetVisibility` (`self.Widget`) true false)
      (`KismetSystemLibrary.RetriggerableDelay` 1.0)
      (set `self.enemydamaged` false))))

(event `self.Box.OnComponentBeginOverlap`
  (params (OverlappedComponent :type "PrimitiveComponent Object Reference") (OtherActor :type "Actor Object Reference") (OtherComp :type "PrimitiveComponent Object Reference") (OtherBodyIndex :type Integer) (bFromSweep :type Boolean) (SweepResult :type "HitResult Structure (by ref)"))
  ;[1 1 1] Attack
  (if (== OtherActor (`GameplayStatics.GetPlayerCharacter` 0))
    (set `self.Attack Mode` true)
    (bind _returnvalue (`KismetSystemLibrary.K2_SetTimerDelegate` (delegate `RangedAttack`) 1.2 true))
    (set `self.AttackEvent` _returnvalue)))

(event `RangedAttack`
  ;[1 1 1] Attack
  (if (not (or (`self.isdead`) (`NavMovementComponent.IsFalling` (`self.CharacterMovement`))))
    (`PaperZDAnimInstance.JumpToNode` (`PaperZDAnimationComponent.AnimInstance` (`self.AnimationComponent`)) (`self.AttackJumpNode`) "None")))

(event `SpawnProjectile`
  ;[1 1 1] Attack
  (`|SpawnActorFromClass` (`self.Projectile`) (`KismetMathLibrary.MakeTransform` (`SceneComponent.K2_GetComponentLocation` (`self.SpawnFireball`)) (`self.K2_GetActorRotation`)) "Undefined" "OverrideRootScale" null null))

(event `self.Box.OnComponentEndOverlap`
  (params (OverlappedComponent :type "PrimitiveComponent Object Reference") (OtherActor :type "Actor Object Reference") (OtherComp :type "PrimitiveComponent Object Reference") (OtherBodyIndex :type Integer))
  ;[1 1 1] Attack
  ;;[1 1 1] Stop attacking when player leaves box
  (if (== OtherActor (`GameplayStatics.GetPlayerCharacter` 0))
    (set `self.Attack Mode` false)
    (`KismetSystemLibrary.K2_ClearAndInvalidateTimerHandle` (`self.AttackEvent`))))

(fn `UserConstructionScript`)